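; Bush ambush point that releases a wolf once enough catchable actors, apparently sheep, gather inside its sphere.
; Sphere overlaps maintain a list of BPI_GetCaught actors, compared against a threshold on each entry.
; The first trigger spawns a hidden BP_Wolf facing the latest entrant, links it to the bush, starts its chase and gamefeel components, and plays leaf effects and sound.
; Later triggers reuse that wolf, hiding it and restarting the chase if idle.
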(event `self.Sphere.OnComponentBeginOverlap`
  (params (OverlappedComponent :type "PrimitiveComponent Object Reference") (OtherActor :type "Actor Object Reference") (OtherComp :type "PrimitiveComponent Object Reference") (OtherBodyIndex :type Integer) (bFromSweep :type Boolean) (SweepResult :type "HitResult Structure (by ref)"))
  (bind _caughtableactorslist (`self.CaughtableActorsList`))
  (bind _wolf (`self.Wolf`))
  (if (`KismetSystemLibrary.DoesImplementInterface` OtherActor "/Game/_Project/Runtime/Code/Interfaces/Wolf/BPI_GetCaught.BPI_GetCaught_C")
    (if (not (`KismetArrayLibrary.Array_Contains` (`self.CaughtableActorsList`) OtherActor))
      (bind _output_get (set `self.Caughtable actor` OtherActor))
      (`KismetArrayLibrary.Array_Add` _caughtableactorslist _output_get))
    (if (>= (`KismetArrayLibrary.Array_Length` _caughtableactorslist) (`self.NbMoutonsPourActiver`))
      (if (`self.hasSpawned`)
        (if (not (`/Game/_Project/Runtime/Code/BP/Wolf/BP_Wolf.isChasing` _wolf))
          (`self.SetActorHiddenInGame` _wolf true)
          (`/Game/_Project/Runtime/Code/BP/Wolf/BP_Wolf.CE_StartChasing` _wolf (`self.ChaseSpeed`)))
        (else
          (set `self.hasSpawned` true)
          (`self.SpawnWolf`)
          (`GameplayStatics.PlaySoundAtLocation` "/Game/_Project/Runtime/Assets/6_Audio/Event/NPC/Wolf/Play_NPC_Wolf_Spawn.Play_NPC_Wolf_Spawn" (0.0 0.0 0.0) (struct) 1.0 1.0 0.0 null null null null))))))

(event `SpawnWolf`
  (bind _wolf (`self.Wolf`))
  (bind _static_mesh (`/Game/_Project/Runtime/Code/BP/Wolf/BP_Wolf.static mesh` _wolf))
  (bind _returnvalue (`|SpawnActorFromClass` "/Game/_Project/Runtime/Code/BP/Wolf/BP_Wolf.BP_Wolf_C" (`KismetAnimationLibrary.K2_LookAt` (`self.GetTransform`) (`self.K2_GetActorLocation` (`self.Caughtable actor`)) (`self.GetActorForwardVector`)) "Undefined" "MultiplyWithRoot" null null))
  (bind _output_get (set `self.Wolf` _returnvalue))
  (`self.SetActorHiddenInGame` _output_get true)
  (set `/Game/_Project/Runtime/Code/BP/Wolf/BP_Wolf.Bush` self _wolf)
  (`/Game/_Project/Runtime/Code/BP/Wolf/BP_Wolf.CE_StartChasing` _wolf (`self.ChaseSpeed`))
  (`GamefeelComponent.InitGamefeelComponent` (`/Game/_Project/Runtime/Code/BP/Wolf/BP_Wolf.BP_JumpyWalkComponent` _wolf) _static_mesh)
  (`GamefeelComponent.InitGamefeelComponent` (`/Game/_Project/Runtime/Code/BP/Wolf/BP_Wolf.BP_WaddlingComponent` _wolf) _static_mesh)
  (`GamefeelComponent.InitGamefeelComponent` (`/Game/_Project/Runtime/Code/BP/Wolf/BP_Wolf.Bp_SquishSquashComponent` _wolf) _static_mesh)
  (`ActorComponent.Activate` (`self.NS_BushLeaves`) true))

(event `self.Sphere.OnComponentEndOverlap`
  (params (OverlappedComponent :type "PrimitiveComponent Object Reference") (OtherActor :type "Actor Object Reference") (OtherComp :type "PrimitiveComponent Object Reference") (OtherBodyIndex :type Integer))
  (if (`KismetSystemLibrary.DoesImplementInterface` OtherActor "/Game/_Project/Runtime/Code/Interfaces/Wolf/BPI_GetCaught.BPI_GetCaught_C")
    (`KismetArrayLibrary.Array_RemoveItem` (`self.CaughtableActorsList`) OtherActor)))

(fn `UserConstructionScript`)