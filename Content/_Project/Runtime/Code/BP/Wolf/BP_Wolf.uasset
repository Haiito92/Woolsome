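; Wolf character that chases and can be bitten, releasing any sheep it carries.
; Starting a chase sets walk speed, flags the AI blackboard and starts jumpy-walk, waddle and squish-squash gamefeel components.
; A bite stops movement and those effects, plays a sound, detaches the caught actor and notifies it through an interface.
; A timer then restores movement and effects and flags the blackboard that the wolf is coming back.
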(event `CE_StartChasing`
  (params (ChaseSpeed :type "Float (double-precision)"))
  (set `self.WolfMaxWalkSpeed` ChaseSpeed)
  (set `CharacterMovementComponent.MaxWalkSpeed` ChaseSpeed (`self.CharacterMovement`))
  (set `self.isChasing` true)
  (`BlackboardComponent.SetValueAsBool` (`AIBlueprintHelperLibrary.GetBlackboard` null) "isChasing" true)
  (`GamefeelComponent.StartGamefeelComponent` (`self.BP_JumpyWalkComponent`))
  (`GamefeelComponent.StartGamefeelComponent` (`self.BP_WaddlingComponent`))
  (`GamefeelComponent.StartGamefeelComponent` (`self.Bp_SquishSquashComponent`)))

(event `self.Bite`
  (params (StunTimer :type "Float (single-precision)"))
  (bind _caughtableactor (`self.CaughtableActor`))
  (bind _caughtableactor_2 (`self.CaughtableActor`))
  (if (not (`self.Bitten`))
    (`GamefeelComponent.StopGamefeelComponent` (`self.BP_JumpyWalkComponent`))
    (`GamefeelComponent.StopGamefeelComponent` (`self.BP_WaddlingComponent`))
    (`GamefeelComponent.StopGamefeelComponent` (`self.Bp_SquishSquashComponent`))
    (set `self.Bitten` true)
    (set `CharacterMovementComponent.MaxWalkSpeed` 0.0 (`self.CharacterMovement`))
    (`self.JUICY_Bitten`)
    (if (`self.SheepAttached`)
      (`self.K2_DetachFromActor` _caughtableactor "KeepWorld" "KeepWorld" "KeepWorld")
      (set `self.SheepAttached` false)
      (`self.SetActorEnableCollision` _caughtableactor true)
      (if (`KismetSystemLibrary.DoesImplementInterface` _caughtableactor_2 "/Game/_Project/Runtime/Code/Interfaces/Wolf/BPI_GetCaught.BPI_GetCaught_C")
        (message `/Game/_Project/Runtime/Code/Interfaces/Wolf/BPI_GetCaught.LetGo` _caughtableactor_2)))
    (`KismetSystemLibrary.K2_SetTimerDelegate` (delegate `Stun`) 2.0)))

(event `Stun`
  (`BlackboardComponent.SetValueAsBool` (`AIBlueprintHelperLibrary.GetBlackboard` null) "isComingBack" true)
  (set `self.Bitten` false)
  (set `CharacterMovementComponent.MaxWalkSpeed` (`self.WolfMaxWalkSpeed`) (`self.CharacterMovement`))
  (`GamefeelComponent.StartGamefeelComponent` (`self.BP_JumpyWalkComponent`))
  (`GamefeelComponent.StartGamefeelComponent` (`self.BP_WaddlingComponent`))
  (`GamefeelComponent.StartGamefeelComponent` (`self.Bp_SquishSquashComponent`)))

(event `JUICY_Bitten`
  ;[1 1 1] JUICY_Bitten
  (`GameplayStatics.SpawnSoundAtLocation` "/Game/_Project/Runtime/Assets/6_Audio/Event/NPC/Wolf/Play_NPC_Wolf_Bite.Play_NPC_Wolf_Bite" (`self.K2_GetActorLocation`) (struct) 1.0 1.0 0.0 null null))

(fn `UserConstructionScript`)