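; Dog (Chien) character Blueprint that adds input, movement juice and bite feedback on top of its parent character.
; BeginPlay initializes jumpy walk, squish-squash and waddling gamefeel components on the static mesh, then start and stop move delegates toggle all three for procedural movement animation.
; Holding input launches a bite and Interacting input launches an interaction.
; The bite juice event plays a bark-bite sound, activates a Niagara effect and prints debug text.
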(event `self.ReceiveBeginPlay`
  (add `StateCharacter.CharacterStartMove_Delegate` (`|CreateDelegate` :!event `OnCharacterStartMove`))
  (add `StateCharacter.CharacterStopMove_Delegate` (`|CreateDelegate` :!event `OnCharacterStopMove`))
  (`|ExecutionSequence`
    (:`then_0`
      (`GamefeelComponent.InitGamefeelComponent` (`self.BP_JumpyWalkComponent`) (`self.StaticMesh`))
      (set `/Game/_Project/Runtime/Code/BP/GameFeel/BP_JumpyWalkComponent.FootstepPoint` (`self.FootstepPoint`) (`self.BP_JumpyWalkComponent`)))
    (:`then_1`
      (`GamefeelComponent.InitGamefeelComponent` (`self.Bp_SquishSquashComponent`) (`self.StaticMesh`)))
    (:`then_2`
      (`GamefeelComponent.InitGamefeelComponent` (`self.BP_WaddlingComponent`) (`self.StaticMesh`)))))

(event `EnhancedInput|/StateMachine/Characters/Common/NewInputs/IA_Characters_Holding`
  (params (ActionValue :type Boolean) (ElapsedSeconds :type "Float (double-precision)") (TriggeredSeconds :type "Float (double-precision)") (InputAction :type "InputAction Object Reference" :default "/StateMachine/Characters/Common/NewInputs/IA_Characters_Holding.IA_Characters_Holding"))
  (:`Started`
    (`self.LaunchBite`)))

(event `EnhancedInput|/StateMachine/Characters/Common/NewInputs/IA_Characters_Interacting`
  (params (ActionValue :type Boolean) (ElapsedSeconds :type "Float (double-precision)") (TriggeredSeconds :type "Float (double-precision)") (InputAction :type "InputAction Object Reference" :default "/StateMachine/Characters/Common/NewInputs/IA_Characters_Interacting.IA_Characters_Interacting"))
  (:`Started`
    (`self.LaunchInteracting`)))

(event `self.JUICY_OnBite`
  (`KismetSystemLibrary.PrintString` "Bite")
  (`GameplayStatics.SpawnSoundAtLocation` "/Game/_Project/Runtime/Assets/6_Audio/Event/MC/MC_Dog/Play_MC_Dog_Bite.Play_MC_Dog_Bite" (`self.K2_GetActorLocation`) (struct) 1.0 1.0 0.0 null null)
  (`ActorComponent.Activate` (`self.NS_Bite`) true))

(event `OnCharacterStartMove`
  (`GamefeelComponent.StartGamefeelComponent` (`self.BP_JumpyWalkComponent`))
  (`GamefeelComponent.StartGamefeelComponent` (`self.Bp_SquishSquashComponent`))
  (`GamefeelComponent.StartGamefeelComponent` (`self.BP_WaddlingComponent`)))

(event `OnCharacterStopMove`
  (`GamefeelComponent.StopGamefeelComponent` (`self.BP_JumpyWalkComponent`))
  (`GamefeelComponent.StopGamefeelComponent` (`self.Bp_SquishSquashComponent`))
  (`GamefeelComponent.StopGamefeelComponent` (`self.BP_WaddlingComponent`)))

(fn `UserConstructionScript`
  (`parent.UserConstructionScript`))